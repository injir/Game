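; CustomAiBp is a minimal AI movement helper that sends a given pawn's AI controller on a simple move and prints a debug message.
; The MovingUnits event and MovingUnit function duplicate this logic separately, scaling the pawn's location or the Blueprint's own location, respectively.
; The goal multiplies that location by a fixed vector, flattening Z to zero, rather than adding an offset.
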(event Custom|MovingUnits
  (params (Pawn :type Basic%20Character%20Object%20Reference))
  (bind _returnvalue (AI|GetAIController Pawn))
  (AI|Navigation|SimpleMovetoLocation _returnvalue (* (Transformation|GetActorLocation Pawn) "200.000000,50.000000, 0"))
  (Development|PrintString "Move"))

(event EventBeginPlay)

(event EventTick
  (params (DeltaSeconds :type Float%20%28single-precision%29)))

(fn ConstructionScript)

(fn MovingUnit
  (params (Pawn :type Basic%20Character%20Object%20Reference))
  (bind _returnvalue (AI|GetAIController Pawn))
  (AI|Navigation|SimpleMovetoLocation _returnvalue (* (Transformation|GetActorLocation) "200.000000,50.000000, 0"))
  (Development|PrintString "Move"))